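; EnemyA_BP is an enemy spawner actor that releases a fixed, timed sequence of waves at its own location.
; On BeginPlay it starts eight one-shot timers, each bound to an EventoOnda event that spawns one enemy at the actor's transform.
; The waves come in pairs of the same class, progressing from EnemyAEsseCaraAqui through Alien2BP and MonstroBP to GoblimBP.
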(event Custom|EventoOnda1
  (Game|SpawnActorfromClass "/Game/MyGame/Inimigo/NewFolder/EnemyAEsseCaraAqui.EnemyAEsseCaraAqui_C" (Transformation|GetActorTransform) "Undefined" 0 0))

(event Custom|EventoOnda3
  (Game|SpawnActorfromClass "/Game/MyGame/Inimigo/NewFolder/Alien2BP.Alien2BP_C" (Transformation|GetActorTransform) "Undefined" 0 0))

(event Custom|EventoOnda2
  (Game|SpawnActorfromClass "/Game/MyGame/Inimigo/NewFolder/EnemyAEsseCaraAqui.EnemyAEsseCaraAqui_C" (Transformation|GetActorTransform) "Undefined" 0 0))

(event Custom|EventoOnda6
  (Game|SpawnActorfromClass "/Game/MyGame/Inimigo/NewFolder/MonstroBP.MonstroBP_C" (Transformation|GetActorTransform) "Undefined" 0 0))

(event Custom|EventoOnda4
  (Game|SpawnActorfromClass "/Game/MyGame/Inimigo/NewFolder/Alien2BP.Alien2BP_C" (Transformation|GetActorTransform) "Undefined" 0 0))

(event Custom|EventoOnda5
  (Game|SpawnActorfromClass "/Game/MyGame/Inimigo/NewFolder/MonstroBP.MonstroBP_C" (Transformation|GetActorTransform) "Undefined" 0 0))

(event Custom|EventoOnda8
  (Game|SpawnActorfromClass "/Game/MyGame/Inimigo/NewFolder/GoblimBP.GoblimBP_C" (Transformation|GetActorTransform) "Undefined" 0 0))

(event Custom|EventoOnda7
  (Game|SpawnActorfromClass "/Game/MyGame/Inimigo/NewFolder/GoblimBP.GoblimBP_C" (Transformation|GetActorTransform) "Undefined" 0 0))

(event EventBeginPlay
  (Utilities|Time|SetTimerbyEvent (delegate Custom|EventoOnda1) 2.0)
  (Utilities|Time|SetTimerbyEvent (delegate Custom|EventoOnda2) 5.0)
  (Utilities|Time|SetTimerbyEvent (delegate Custom|EventoOnda3) 16.0)
  (Utilities|Time|SetTimerbyEvent (delegate Custom|EventoOnda4) 19.0)
  (Utilities|Time|SetTimerbyEvent (delegate Custom|EventoOnda5) 3e+01)
  (Utilities|Time|SetTimerbyEvent (delegate Custom|EventoOnda6) 33.0)
  (Utilities|Time|SetTimerbyEvent (delegate Custom|EventoOnda7) 4e+01)
  (Utilities|Time|SetTimerbyEvent (delegate Custom|EventoOnda8) 43.0))

(event Collision|EventActorBeginOverlap
  (params (OtherActor :type Actor%20Object%20Reference)))

(event EventTick
  (params (DeltaSeconds :type Float%20%28single-precision%29)))

(fn ConstructionScript)