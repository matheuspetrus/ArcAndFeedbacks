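; MonstroBP is an enemy monster that chases and attacks the first-person player.
; It turns to face the player every tick, and PawnSensing sightings of the player trigger an AIMoveTo toward them.
; Hits with the player set the Ataque flag from SelfMoved and print its state.
; PerderVida sets health (Vida) to the passed VidaInimigo minus current Vida, with no death handling here.
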(event OnSeePawn(PawnSensing)
  (params (Pawn :type Pawn%20Object%20Reference))
  (Utilities|Casting|CastToFirstPersonCharacter Pawn)
  (AI|AIMoveTo self "0, 0, 0" (Game|GetPlayerCharacter 0) 5.0 false))

(event Collision|EventHit
  (params (MyComp :type Primitive%20Component%20Object%20Reference) (Other :type Actor%20Object%20Reference) (OtherComp :type Primitive%20Component%20Object%20Reference) (bSelfMoved :type Boolean) (HitLocation :type Vector :default "0, 0, 0") (HitNormal :type Vector :default "0, 0, 0") (NormalImpulse :type Vector :default "0, 0, 0") (Hit :type Hit%20Result%20Structure%20%28by%20ref%29))
  (Utilities|Casting|CastToFirstPersonCharacter Other)
  (if bSelfMoved
    (Variables|Default|Setataque true)
    (Development|PrintString "Ataque verdadeiro")
    (else
      (Variables|Default|Setataque false)
      (Development|PrintString "Ataque falso"))))

(event Collision|EventActorBeginOverlap
  (params (OtherActor :type Actor%20Object%20Reference)))

(event EventTick
  (params (DeltaSeconds :type Float%20%28single-precision%29))
  (Transformation|SetActorRotation (Math|Rotator|FindLookatRotation (Transformation|GetWorldLocation (Variables|Collision|GetCapsuleComponent)) (Transformation|GetActorLocation (Game|GetPlayerCharacter 0)))))

(event EventBeginPlay
  (Variables|Default|SetVida 1.0)
  (Class|PawnSensingComponent|SetSensingUpdatesEnabled (Variables|Pawn|GetPawnSensing) true))

(fn ConstructionScript)

(fn PerderVida
  (params (VidaInimigo :type Float%20%28single-precision%29))
  (Variables|Default|SetVida (- VidaInimigo (Variables|Default|GetVida))))