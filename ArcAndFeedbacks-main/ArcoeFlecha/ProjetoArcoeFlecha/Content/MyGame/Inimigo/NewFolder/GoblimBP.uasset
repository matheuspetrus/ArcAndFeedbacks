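; Goblin enemy character Blueprint that chases and attacks the first-person player.
; Every Tick it rotates to face the player, and when PawnSensing sees the player it starts an AI MoveTo toward them.
; Move success sets the Ataque flag on its Goblim_Anim instance, and failure clears it.
; Vida starts at full on BeginPlay, and PerderVida sets it to the passed value minus current Vida, with no death handling.
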(event OnSeePawn(PawnSensing)
  (params (Pawn :type Pawn%20Object%20Reference))
  (Utilities|Casting|CastToFirstPersonCharacter Pawn)
  (AI|AIMoveTo self "0, 0, 0" (Game|GetPlayerCharacter 0) 5.0 false
    (:OnSuccess
      (bind _asgoblim_anim (Utilities|Casting|CastToGoblim_Anim (Components|SkeletalMesh|GetAnimInstance (Variables|Character|GetMesh))))
      (Variables|/Game/MyGame/Inimigo/NewFolder/Goblim_Anim.Goblim_Anim_C|SetAtaque _asgoblim_anim true))
    (:OnFail
      (bind _asgoblim_anim_2 (Utilities|Casting|CastToGoblim_Anim (Components|SkeletalMesh|GetAnimInstance (Variables|Character|GetMesh))))
      (Variables|/Game/MyGame/Inimigo/NewFolder/Goblim_Anim.Goblim_Anim_C|SetAtaque _asgoblim_anim_2 false))))

(event Collision|EventActorBeginOverlap
  (params (OtherActor :type Actor%20Object%20Reference)))

(event EventTick
  (params (DeltaSeconds :type Float%20%28single-precision%29))
  (Transformation|SetActorRotation (Math|Rotator|FindLookatRotation (Transformation|GetWorldLocation (Variables|Collision|GetCapsuleComponent)) (Transformation|GetActorLocation (Game|GetPlayerCharacter 0)))))

(event EventBeginPlay
  (Variables|Default|SetVida 1.0)
  (Class|PawnSensingComponent|SetSensingUpdatesEnabled (Variables|Pawn|GetPawnSensing) true))

(fn ConstructionScript)

(fn PerderVida
  (params (VidaInimigo :type Float%20%28single-precision%29))
  (Variables|Default|SetVida (- VidaInimigo (Variables|Default|GetVida))))